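; Spawner actor that turns the player's card hand into moving rhythm notes for the action phase.
; On BeginPlay it looks up each hand card in DT_CardTable and spawns its notes at their offsets, one bar-length apart per card.
; Each left, right or both note receives its card and a projectile velocity.
; A missed-note counter binds to the player controller, while hand initialization is an empty stub.
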(event `self.ReceiveBeginPlay`
  (bind _asbp_action_phase_player_controller (cast `/Game/Blueprints/BP_ActionPhase_PlayerController` (`GameplayStatics.GetPlayerController` 0)))
  (add `/Game/Blueprints/BP_ActionPhase_PlayerController.OnNoteMissed` _asbp_action_phase_player_controller (delegate `IncrementNotesMissed`))
  (`self.InitializeHand`)
  ;[1 1 1] Represents bar length (1000 units = 1 bar)
  (set `self.CardOffset` 1000.0)
  (set `self.SpawnVelocity` (0.0 -250.0 0.0))
  (`self.SpawnCardsFromHand` (`PlayerStats.playerHand` (subsystem `PlayerStats`))))

(event `IncrementNotesMissed`
  (params (Card :type "/Game/Blueprints/DataTables/F_CardStructure Structure") (Name :type Name))
  (`/Engine/EditorBlueprintResources/StandardMacros.IncrementInt` (`self.NotesMissed`)))

(fn `InitializeHand`)

(fn `Spawn`
  (params (NoteClass :type "Actor Class Reference") (Offset :type "Float (double-precision)"))
  (bind (_returnvalue_location _returnvalue_rotation) (`KismetMathLibrary.BreakTransform` (`self.GetTransform`)))
  (bind _currentcard (`self.CurrentCard`))
  (bind _spawnvelocity (`self.SpawnVelocity`))
  (bind _noteobject (`self.NoteObject`))
  (bind _returnvalue (`|SpawnActorFromClass` NoteClass (`KismetMathLibrary.MakeTransform` (+ _returnvalue_location (`KismetMathLibrary.MakeVector` 0.0 Offset)) _returnvalue_rotation (`self.SpawnScale`)) "Undefined" "OverrideRootScale" null null))
  (set `self.NoteObject` _returnvalue)
  ;[1 1 1] Figure out which note's projectile movment component to grab
  (bind _asbp_left_note (cast `/Game/Blueprints/BP_LeftNote` _noteobject)
    (:`then`
      (set `/Game/Blueprints/BP_LeftNote.Card` _currentcard _asbp_left_note)
      (`ProjectileMovementComponent.SetVelocityInLocalSpace` (`/Game/Blueprints/BP_LeftNote.ProjectileMovement` _asbp_left_note) _spawnvelocity))
    (:`CastFailed`
      (bind _asbp_right_note (cast `/Game/Blueprints/BP_RightNote` _noteobject)
        (:`then`
          (set `/Game/Blueprints/BP_RightNote.Card` _currentcard _asbp_right_note)
          (`ProjectileMovementComponent.SetVelocityInLocalSpace` (`/Game/Blueprints/BP_RightNote.ProjectileMovement` _asbp_right_note) _spawnvelocity))
        (:`CastFailed`
          (bind _asbp_both_note (cast `/Game/Blueprints/BP_BothNote` _noteobject))
          (set `/Game/Blueprints/BP_BothNote.Card` _currentcard _asbp_both_note)
          (`ProjectileMovementComponent.SetVelocityInLocalSpace` (`/Game/Blueprints/BP_BothNote.ProjectileMovement` _asbp_both_note) _spawnvelocity))))))

(fn `SpawnCardsFromHand`
  (params (Hand :type "Array of Name"))
  (for (_array_element _array_index) Hand
    (bind _returnvalue (`|GetDataTableRow` "/Game/Blueprints/DataTables/DT_CardTable.DT_CardTable" _array_element)
      (:`then`
        (bind _output_get (set `self.CurrentCard` _returnvalue))
        (set `self.NotesMissed` 0)
        (`self.SpawnNotesFromCard` (`.Notes_29_E2D9BC2C4091FD2748348EA87304AACA` (break `/Game/Blueprints/DataTables/F_CardStructure` _output_get)) (`.Offset_28_733363A747BA322D47F7DEA0ED58D10A` (break `/Game/Blueprints/DataTables/F_CardStructure` _output_get)) (* _array_index (`self.CardOffset`))))
      (:`RowNotFound`
        (`KismetSystemLibrary.PrintString` "Row not found")))))

(fn `SpawnNotesFromCard`
  (params (Notes :type "Array of Actor Class Reference") (Offsets :type "Array of Float (double-precision)") (CardOffset :type "Float (double-precision)"))
  ;[1 1 1] This function exists purlely to allow for loops during testing
  (for (_array_element _array_index) Notes
    (`self.Spawn` _array_element (+ (`|GetArrayItem` Offsets _array_index) CardOffset)))
  (bind _output_get (set `self.NotesMissed` 0))
  (bind _output_get_2 (set `self.PercentageCorrect` (`KismetMathLibrary.Conv_IntToDouble` (/ _output_get (`KismetArrayLibrary.Array_Length` (`self.Notes`))))))
  (`KismetSystemLibrary.PrintString` (`KismetStringLibrary.Conv_DoubleToString` _output_get_2)))

(fn `UserConstructionScript`)