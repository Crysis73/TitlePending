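; BP_GoodZone is the rhythm-game hit zone that checks left and right button presses against incoming notes during the action phase.
; PerfectBox overlaps store the latest left, right or both note and its card, with no end-overlap clearing.
; Player controller events latch button flags until a hit or miss resets them.
; A matching combination (one side alone, or both for both notes) reports the card as played and destroys the note.
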(event `self.PerfectBox.OnComponentBeginOverlap`
  (params (OverlappedComponent :type "PrimitiveComponent Object Reference") (OtherActor :type "Actor Object Reference") (OtherComp :type "PrimitiveComponent Object Reference") (OtherBodyIndex :type Integer) (bFromSweep :type Boolean) (SweepResult :type "HitResult Structure (by ref)"))
  (`self.DetermineOverlappedActor` OtherActor))

(event `self.ReceiveBeginPlay`
  (bind _playercontroller (`self.PlayerController`))
  (bind _asbp_action_phase_player_controller (cast `/Game/Blueprints/BP_ActionPhase_PlayerController` (`GameplayStatics.GetPlayerController` 0)))
  (set `self.PlayerController` _asbp_action_phase_player_controller)
  (add `/Game/Blueprints/BP_ActionPhase_PlayerController.OnLeftBtnPressed` _playercontroller (delegate `HandleLeftBtn`))
  (add `/Game/Blueprints/BP_ActionPhase_PlayerController.OnRightBtnPressed` _playercontroller (delegate `HandleRightBtn`))
  (add `/Game/Blueprints/BP_ActionPhase_PlayerController.OnNoteMissed` _playercontroller (delegate `ClearBtnInput`)))

(event `HandleLeftBtn`
  (set `self.LeftRecieved` true)
  (`self.HandleButtonInput` "L"))

(event `HandleRightBtn`
  (set `self.RightRecieved` true)
  (`self.HandleButtonInput` "R"))

(event `ClearBtnInput`
  (params (Card :type "/Game/Blueprints/DataTables/F_CardStructure Structure") (Name :type Name))
  (set `self.LeftRecieved` false)
  (set `self.RightRecieved` false))

(fn `CallNotePlayed`
  (`/Game/Blueprints/BP_ActionPhase_PlayerController.OnNotePlayed` (`self.PlayerController`) (`self.CurrentCard`) "None")
  (set `self.LeftRecieved` false)
  (set `self.RightRecieved` false)
  (`self.K2_DestroyActor` (`self.NoteInPlayzone`)))

(fn `DetermineOverlappedActor`
  (params (Actor :type "Actor Object Reference"))
  (bind _asbp_left_note (cast `/Game/Blueprints/BP_LeftNote` Actor)
    (:`then`
      (set `self.NoteInPlayzone` _asbp_left_note)
      (set `self.CurrentCard` (`/Game/Blueprints/BP_LeftNote.Card` _asbp_left_note)))
    (:`CastFailed`
      (bind _asbp_right_note (cast `/Game/Blueprints/BP_RightNote` Actor)
        (:`then`
          (set `self.NoteInPlayzone` _asbp_right_note)
          (set `self.CurrentCard` (`/Game/Blueprints/BP_RightNote.Card` _asbp_right_note)))
        (:`CastFailed`
          (bind _asbp_both_note (cast `/Game/Blueprints/BP_BothNote` Actor))
          (set `self.NoteInPlayzone` _asbp_both_note)
          (set `self.CurrentCard` (`/Game/Blueprints/BP_BothNote.Card` _asbp_both_note)))))))

(fn `HandleButtonInput`
  (params (Side :type String))
  (bind _returnvalue (`GameplayStatics.GetObjectClass` (`self.NoteInPlayzone`)))
  (if (== _returnvalue "/Game/Blueprints/BP_BothNote.BP_BothNote_C")
    (if (and (`self.RightRecieved`) (`self.LeftRecieved`))
      (`self.CallNotePlayed`))
    (elif (== _returnvalue "/Game/Blueprints/BP_RightNote.BP_RightNote_C")
      (if (and (`self.RightRecieved`) (not (`self.LeftRecieved`)))
        (`self.CallNotePlayed`))
      (elif (== _returnvalue "/Game/Blueprints/BP_LeftNote.BP_LeftNote_C")
        (if (and (`self.LeftRecieved`) (not (`self.RightRecieved`)))
          (`self.CallNotePlayed`))
        (else
          (`KismetSystemLibrary.PrintString` "No note in playzone"))))))

(fn `Print`
  (params (NoteType :type String) (Box :type String))
  (`KismetSystemLibrary.PrintString` (`KismetStringLibrary.Concat_StrStr` NoteType " in" Box)))

(fn `UserConstructionScript`)