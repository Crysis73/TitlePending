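; Player controller for the action phase of a rhythm card game, turning played and missed notes into card effects.
; It creates the player interface and stats HUD, relays button presses, and tallies notes per card, switching cards when a different one arrives.
; A completed card is scored as fail, partial or success to set its damage, armor or healing, then ends the turn.
; Incoming damage reduces player health and opens LoseScreen at zero.
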(event `self.ReceiveBeginPlay`
  (`self.InitializeUIVars`)
  (add `Button.OnPressed` (`self.LeftBtn`) (delegate `LeftBtnPressed`))
  (add `Button.OnPressed` (`self.RightBtn`) (delegate `RightBtnPressed`))
  (add `self.OnNotePlayed` (delegate `NotePlayed`))
  (add `self.OnNoteMissed` (delegate `NoteMissed`))
  (`UserWidget.AddToViewport` (`self.PlayerUI`) 0)
  (add `self.CardChanged` (delegate `OnCardChanged`))
  (`self.InitializeHealthBars`)
  (add `self.PlayerDamaged` (delegate `OnPlayerDamaged`))
  (add `self.OnExecutionDetermined` (delegate `CardEffect`)))

(event `LeftBtnPressed`
  (`self.OnLeftBtnPressed`))

(event `RightBtnPressed`
  (`self.OnRightBtnPressed`))

(event `NotePlayed` :!signature `self.OnNotePlayed`
  (params (Card :type "/Game/Blueprints/DataTables/F_CardStructure Structure") (Name :type Name))
  (`self.HandleNoteEvents` Card))

(event `NoteMissed` :!signature `self.OnNoteMissed`
  (params (Card :type "/Game/Blueprints/DataTables/F_CardStructure Structure") (Name :type Name))
  (`self.HandleNoteEvents` Card true))

(event `CardEffect` :!signature `self.OnExecutionDetermined`
  (params (PercentageCorrect :type "Float (double-precision)") (ExecutionScore :type Integer) (Card :type "/Game/Blueprints/DataTables/F_CardStructure Structure"))
  (`self.ApplyCardEffect` Card ExecutionScore)
  (`KismetSystemLibrary.PrintString` (`KismetStringLibrary.Conv_IntToString` ExecutionScore) true true (struct :`R` 1.0 :`G` 0.41457 :`B` 0.366773 :`A` 1.0))
  (`self.PlayerTurnTaken`))

(event `OnPlayerDamaged` :!signature `self.PlayerDamaged`
  (params (Damage :type Integer))
  (`self.DamagePlayer` Damage))

(event `OnCardChanged`
  (`self.HandleCardChanged` (`self.PlayerUI`)))

(fn `ApplyCardEffect`
  (params (Card :type "/Game/Blueprints/DataTables/F_CardStructure Structure") (Execution :type Integer))
  (bind _returnvalue (subsystem `PlayerStats`))
  (switch `string` Card_Type_8_1E0703B94F02174D5996068830E6116F
    (:`Attack`
      (switch `int` Execution
        (:`0`
          (`self.DamageEnemy` Card_ValueFail_20_CABB3F4B4FC198DE2BA164B02552AB06))
        (:`1`
          (`self.DamageEnemy` Card_ValuePartial_18_C461449146934529E91B5580F26020A8))
        (:`2`
          (`self.DamageEnemy` Card_ValueSuccess_21_0842977347F5FD1895A8FBA131177635))))
    (:`Defense`
      (switch `int` Execution
        (:`0`
          (`PlayerStats.AddArmor` _returnvalue Card_ValueFail_20_CABB3F4B4FC198DE2BA164B02552AB06))
        (:`1`
          (`PlayerStats.AddArmor` _returnvalue Card_ValuePartial_18_C461449146934529E91B5580F26020A8))
        (:`2`
          (`PlayerStats.AddArmor` _returnvalue Card_ValueSuccess_21_0842977347F5FD1895A8FBA131177635))))
    (:`Utility`
      (switch `int` Execution
        (:`0`
          (`PlayerStats.HealDamage` _returnvalue Card_ValueFail_20_CABB3F4B4FC198DE2BA164B02552AB06))
        (:`1`
          (`PlayerStats.HealDamage` _returnvalue Card_ValuePartial_18_C461449146934529E91B5580F26020A8))
        (:`2`
          (`PlayerStats.HealDamage` _returnvalue Card_ValueSuccess_21_0842977347F5FD1895A8FBA131177635))))))

(fn `DamagePlayer`
  (params (Damage :type Integer))
  (bind _returnvalue (subsystem `PlayerStats`))
  (`PlayerStats.TakeDamage` _returnvalue Damage)
  (if (<= (`PlayerStats.CurrentHealth` _returnvalue) 0)
    (`GameplayStatics.OpenLevel` "LoseScreen")))

(fn `DetermineLastNote`
  (bind (_currentcard_name _currentcard_type _currentcard_valuefail _currentcard_valuepartial _currentcard_valuesuccess _currentcard_notes) (break `/Game/Blueprints/DataTables/F_CardStructure` (`self.CurrentCard`)))
  (bind _result (`/Engine/EditorBlueprintResources/StandardMacros.IncrementInt` (`self.Notes`))
    (:`  `
      (if (== _result (`KismetArrayLibrary.Array_Length` _currentcard_notes))
        (`self.GetPercentageCorrect`)))))

(fn `EnemyAction`
  (bind _targetedenemy (`self.TargetedEnemy`))
  (for _ (range 5)
    (`KismetArrayLibrary.Array_Add` (`self.EnemyActionType`) (`KismetMathLibrary.RandomInteger` 3))
    (`KismetSystemLibrary.PrintString` "AddedElement"))
  (for _array_element (`self.EnemyActionType`)
    (if (== _array_element 1)
      (`self.DamagePlayer` 0)
      (else
        (set `/Game/Blueprints/BP_EnemyIcon.Armor` (+ (`/Game/Blueprints/BP_EnemyIcon.Armor` _targetedenemy) (`/Game/Blueprints/BP_EnemyIcon.Defense` _targetedenemy)) _targetedenemy)))))

(fn `GetPercentageCorrect`
  (returns (PercentageCorrect :type "Float (double-precision)") (ExecutionScore :type Integer))
  (bind (_currentcard_name _currentcard_type _currentcard_valuefail _currentcard_valuepartial _currentcard_valuesuccess _currentcard_notes) (break `/Game/Blueprints/DataTables/F_CardStructure` (`self.CurrentCard`)))
  (bind _returnvalue (`KismetArrayLibrary.Array_Length` _currentcard_notes))
  (bind _returnvalue_2 (`KismetMathLibrary.Conv_IntToDouble` (/ (- _returnvalue (`self.NotesMissed`)) _returnvalue)))
  (if (`KismetMathLibrary.InRange_FloatFloat` _returnvalue_2 0.0 0.5 true false)
    (return _returnvalue_2 0)
    (elif (`KismetMathLibrary.InRange_FloatFloat` _returnvalue_2 0.5 0.75 true false)
      (return _returnvalue_2 1)
      (else
        (return _returnvalue_2 2)))))

(fn `HandleCardChanged`
  (params (UI :type "/Game/Blueprints/Widgets/WBP_ActionPhase_PlayerInterface Object Reference"))
  (bind (_currentcard_name _currentcard_type _currentcard_valuefail _currentcard_valuepartial _currentcard_valuesuccess _currentcard_notes _currentcard_offset _currentcard_image) (break `/Game/Blueprints/DataTables/F_CardStructure` (`self.CurrentCard`)))
  (`Image.SetBrush` (`/Game/Blueprints/Widgets/WBP_ActionPhase_PlayerInterface.CurrentCardImg` UI) (`WidgetBlueprintLibrary.MakeBrushFromAsset` _currentcard_image)))

(fn `HandleNoteEvents`
  (params (Card :type "/Game/Blueprints/DataTables/F_CardStructure Structure") (NoteMissed :type Boolean))
  (locals (NoteIsMissed :type Boolean) (PotentialCard :type "/Game/Blueprints/DataTables/F_CardStructure Structure"))
  (bind _notes (`self.Notes`))
  (bind (_currentcard_name _currentcard_type _currentcard_valuefail _currentcard_valuepartial _currentcard_valuesuccess _currentcard_notes) (break `/Game/Blueprints/DataTables/F_CardStructure` (`self.CurrentCard`)))
  (set `local.NoteIsMissed` NoteMissed)
  (set `local.PotentialCard` Card)
  (if (== (`.Name_7_6322F13A4315B1FDE615E09F214F98A1` (break `/Game/Blueprints/DataTables/F_CardStructure` Card)) (`.Name_7_6322F13A4315B1FDE615E09F214F98A1` (break `/Game/Blueprints/DataTables/F_CardStructure` (`self.CurrentCard`))))
    (`|ExecutionSequence`
      (:`then_0`
        (`/Engine/EditorBlueprintResources/StandardMacros.IncrementInt` _notes
          (:`  `
            (if (== (`KismetArrayLibrary.Array_Length` _currentcard_notes) _notes)
              (bind (_percentagecorrect _executionscore) (`self.GetPercentageCorrect`))
              (`KismetSystemLibrary.PrintString` "Called on execution determined")
              (`self.OnExecutionDetermined` _percentagecorrect _executionscore (`self.CurrentCard`))))))
      (:`then_1`
        (if (`local.NoteIsMissed`)
          (`/Engine/EditorBlueprintResources/StandardMacros.IncrementInt` (`self.NotesMissed`)))))
    (else
      ;[1 1 1] TODO: Refactor into function
      (set `self.Notes` 1)
      (set `self.CurrentCard` (`local.PotentialCard`))
      (set `self.NotesMissed` (`KismetMathLibrary.Conv_BoolToInt` (`local.NoteIsMissed`)))
      (`self.CardChanged`))))

(fn `InitializeHealthBars`
  (bind _returnvalue (`|CreateWidget` "/Game/Blueprints/Widgets/WBP_StatsHUD.WBP_StatsHUD_C"))
  (`UserWidget.AddToViewport` _returnvalue 0))

(fn `InitializeUIVars`
  (bind _returnvalue (`|CreateWidget` "/Game/Blueprints/Widgets/WBP_ActionPhase_PlayerInterface.WBP_ActionPhase_PlayerInterface_C"))
  (bind _output_get (set `self.PlayerUI` _returnvalue))
  (set `self.LeftBtn` (`/Game/Blueprints/Widgets/WBP_ActionPhase_PlayerInterface.LeftBtn` _output_get))
  (set `self.RightBtn` (`/Game/Blueprints/Widgets/WBP_ActionPhase_PlayerInterface.RightBtn` _output_get)))

(fn `UserConstructionScript`)