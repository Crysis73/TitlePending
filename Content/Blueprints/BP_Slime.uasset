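; BP_Slime is the action-phase slime, a flipbook sprite that reacts to the player's correct inputs.
; On BeginPlay it binds UpdateAnimation to the action-phase player controller's OnPlayerCorrect event.
; AnimStateMachine picks the Damaged flipbook while the controller's Success count is below two, otherwise Death.
; A short timer returns the sprite to Idle after damage.
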(event `self.ReceiveBeginPlay`
  (bind _asbp_action_phase_player_controller (cast `/Game/Blueprints/BP_ActionPhase_PlayerController` (`GameplayStatics.GetPlayerController` 0)))
  (add `/Game/Blueprints/BP_ActionPhase_PlayerController.OnPlayerCorrect` _asbp_action_phase_player_controller (delegate `Update Animation`)))

(event `Update Animation`
  (`KismetSystemLibrary.K2_SetTimer` null "Anim State Machine" 0.5)
  (bind _paperflipbook (`self.AnimStateMachine` (`/Game/Blueprints/BP_ActionPhase_PlayerController.Success` (stale `self.ReceiveBeginPlay` _asbp_action_phase_player_controller))))
  (`PaperFlipbookComponent.SetFlipbook` (`self.SpriteReal`) _paperflipbook))

(fn `AnimStateMachine`
  (params (PlayerSuccess :type Integer))
  (returns (PaperFlipbook :type "PaperFlipbook Object Reference"))
  (if (< PlayerSuccess 2)
    ;[1 1 1] Timer for resetting to idle animation after damaged animation is called
    (`KismetSystemLibrary.K2_SetTimer` null "ResetAnimation" 0.5)
    (set `self.AnimationState` "NewEnumerator1")
    (else
      (set `self.AnimationState` "NewEnumerator2")))
  (return (select `/Game/Sprites/Slime/AnimationState` (`self.AnimationState`) :`NewEnumerator0` (`self.IdleFlipbook`) :`NewEnumerator1` (`self.DamagedFlipbook`) :`NewEnumerator2` (`self.DeathFlipbook`))))

(fn `ResetAnimation`
  (`PaperFlipbookComponent.SetFlipbook` (`self.SpriteReal`) (`self.IdleFlipbook`)))

(fn `UserConstructionScript`)