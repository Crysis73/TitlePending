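; Player controller for the planning phase that builds the player's card hand and displays it on screen.
; On BeginPlay it resets and reinitializes the PlayerStats deck, then appends each card's DT_CardTable row to CaseyHand.
; It passes CaseyHand to a new WBP_PlayerHand widget in the viewport.
; SetPlayerHand copies a separate Hand variable into PlayerStats but is not called within this graph.
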(event `self.ReceiveBeginPlay`
  (`self.DrawNewHand`)
  (`self.InitializeWidgets`))

(fn `DrawNewHand`
  (bind _returnvalue (subsystem `PlayerStats`))
  (`PlayerStats.ObliterateDeck` _returnvalue) ; Eventually will occur once per gameplay Loop
  (`PlayerStats.InitializeDeck` _returnvalue)
  (for _array_element (`PlayerStats.playerDeck` _returnvalue)
    (bind _returnvalue_2 (`|GetDataTableRow` "/Game/Blueprints/DataTables/DT_CardTable.DT_CardTable" _array_element)
      (:`then`
        (`KismetArrayLibrary.Array_Append` (`self.CaseyHand`) (`|MakeArray` _returnvalue_2))))))

(fn `InitializeWidgets`
  (bind _returnvalue (`|CreateWidget` "/Game/Blueprints/Widgets/WBP_PlayerHand.WBP_PlayerHand_C" (`GameplayStatics.GetPlayerController` 0) (`self.CaseyHand`)))
  (`UserWidget.AddToViewport` _returnvalue 0))

(fn `SetPlayerHand`
  (set `PlayerStats.playerHand` (`self.Hand`) (subsystem `PlayerStats`)))

(fn `UserConstructionScript`)