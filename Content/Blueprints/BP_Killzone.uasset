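; Kill zone for a note-based action phase that registers missed notes and removes them.
; On box overlap, a helper casts the actor to left, right or both note and stores it with its card.
; The event then reports the stored card as missed to the action-phase player controller and destroys the stored note.
; Non-note overlaps are not filtered, so the event still runs on the previously stored values.
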(event `self.ReceiveActorBeginOverlap`
  (params (OtherActor :type "Actor Object Reference")))

(event `self.Box.OnComponentBeginOverlap`
  (params (OverlappedComponent :type "PrimitiveComponent Object Reference") (OtherActor :type "Actor Object Reference") (OtherComp :type "PrimitiveComponent Object Reference") (OtherBodyIndex :type Integer) (bFromSweep :type Boolean) (SweepResult :type "HitResult Structure (by ref)"))
  (`self.Determine Overlapped Actor` OtherActor)
  (bind _asbp_action_phase_player_controller (cast `/Game/Blueprints/BP_ActionPhase_PlayerController` (`GameplayStatics.GetPlayerController` 0)))
  (`/Game/Blueprints/BP_ActionPhase_PlayerController.OnNoteMissed` _asbp_action_phase_player_controller (`self.CurrentCard`) "None")
  (`self.K2_DestroyActor` (`self.NoteInPlayzone`)))

(fn `Determine Overlapped Actor`
  (params (Actor :type "Actor Object Reference"))
  (bind _asbp_left_note (cast `/Game/Blueprints/BP_LeftNote` Actor)
    (:`then`
      (set `self.NoteInPlayzone` _asbp_left_note)
      (set `self.CurrentCard` (`/Game/Blueprints/BP_LeftNote.Card` _asbp_left_note)))
    (:`CastFailed`
      (bind _asbp_right_note (cast `/Game/Blueprints/BP_RightNote` Actor)
        (:`then`
          (set `self.NoteInPlayzone` _asbp_right_note)
          (set `self.CurrentCard` (`/Game/Blueprints/BP_RightNote.Card` _asbp_right_note)))
        (:`CastFailed`
          (bind _asbp_both_note (cast `/Game/Blueprints/BP_BothNote` Actor))
          (set `self.NoteInPlayzone` _asbp_both_note)
          (set `self.CurrentCard` (`/Game/Blueprints/BP_BothNote.Card` _asbp_both_note)))))))

(fn `UserConstructionScript`)