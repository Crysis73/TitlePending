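; Enemy actor for the card battle's action phase, initialized from a random DT_EnemyInfo row with stats, flipbooks and actions.
; On the player controller's turn-taken event, it always plays its first action: attack, block or heal.
; Damage events lower health and switch to a damaged flipbook, reset by timer, or a death one.
; The win check subtracts damage a second time before opening WinScreen, so it can trigger early.
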(event `self.ReceiveBeginPlay`
  (`self.InitializeEnemy`)
  (bind _asbp_action_phase_player_controller (cast `/Game/Blueprints/BP_ActionPhase_PlayerController` (`GameplayStatics.GetPlayerController` 0)))
  (add `/Game/Blueprints/BP_ActionPhase_PlayerController.PlayerTurnTaken` _asbp_action_phase_player_controller (delegate `OnPlayerTurnTaken`))
  (add `/Game/Blueprints/BP_ActionPhase_PlayerController.DamageEnemy` _asbp_action_phase_player_controller (delegate `OnEnemyDamaged`)))

(event `OnEnemyDamaged`
  (params (Damage :type Integer))
  (`self.DamageEnemy` Damage)
  (bind _paperflipbook (`self.AnimStateMachine`))
  (`PaperFlipbookComponent.SetFlipbook` (`self.EnemySprite`) _paperflipbook))

(event `OnPlayerTurnTaken`
  (`self.TakeEnemyTurn`))

(fn `AnimStateMachine`
  (returns (PaperFlipbook :type "PaperFlipbook Object Reference"))
  (if (> (`self.CurrentHealth`) 0)
    ;[1 1 1] Timer for resetting to idle animation after damaged animation is called
    (`KismetSystemLibrary.K2_SetTimer` null "ResetAnimation" 0.5)
    (set `self.AnimationState` "NewEnumerator1")
    (else
      (set `self.AnimationState` "NewEnumerator2")))
  (return (select `/Game/Sprites/Slime/AnimationState` (`self.AnimationState`) :`NewEnumerator0` (`self.IdleFlipbook`) :`NewEnumerator1` (`self.DamagedFlipbook`) :`NewEnumerator2` (`self.DeathFlipbook`))))

(fn `ApplyCardEffect`
  (params (Card :type String))
  (locals (CardName :type String) (CardValue :type Integer) (CardFound :type Boolean :default false) (PlayerController :type "/Game/Blueprints/BP_ActionPhase_PlayerController Object Reference"))
  (bind _cardfound (`local.CardFound`))
  (bind (_value _returnvalue) (`BlueprintMapLibrary.Map_Find` (`self.Actions`) (`local.CardName`)))
  (set `local.CardName` Card)
  (bind _asbp_action_phase_player_controller (cast `/Game/Blueprints/BP_ActionPhase_PlayerController` (`GameplayStatics.GetPlayerController` 0)))
  (set `local.PlayerController` _asbp_action_phase_player_controller)
  (set `local.CardValue` _value)
  (set `local.CardFound` _returnvalue)
  (switch `string` (`local.CardName`)
    (:`Attack`
      (if _cardfound
        (`KismetSystemLibrary.PrintString` "Attacking Player")
        (`/Game/Blueprints/BP_ActionPhase_PlayerController.PlayerDamaged` (`local.PlayerController`) (`local.CardValue`))
        (else
          (`KismetSystemLibrary.PrintString` "Failed to attack player"))))
    (:`Block`
      (if _cardfound
        (bind _output_get (set `self.Armor` (+ (stale _output_get) (`local.CardValue`))))
        (`KismetSystemLibrary.PrintString` "Enemy Blocking")
        (else
          (`KismetSystemLibrary.PrintString` "Failed to block"))))
    (:`Heal`
      (if _cardfound
        (bind _returnvalue_2 (+ (stale _output_get_2) (`local.CardValue`)))
        (bind _output_get_2 (set `self.CurrentHealth` _returnvalue_2))
        (`KismetSystemLibrary.PrintString` "Enemy Healing")
        (if (>= _returnvalue_2 (`self.MaxHealth`))
          (set `self.CurrentHealth` (`self.MaxHealth`)))
        (else
          (`KismetSystemLibrary.PrintString` "Failed to heal"))))))

(fn `DamageEnemy`
  (params (Damage :type Integer))
  (bind _returnvalue (- (stale _output_get) Damage))
  (bind _output_get (set `self.CurrentHealth` _returnvalue))
  (if (<= _returnvalue 0)
    (`GameplayStatics.OpenLevel` "WinScreen")))

(fn `InitializeEnemy`
  (bind _outrownames (`DataTableFunctionLibrary.GetDataTableRowNames` "/Game/Blueprints/DataTables/DT_EnemyInfo.DT_EnemyInfo"))
  (bind _returnvalue (`|GetDataTableRow` "/Game/Blueprints/DataTables/DT_EnemyInfo.DT_EnemyInfo" (`|GetArrayItem` _outrownames (`KismetMathLibrary.RandomInteger` (`KismetArrayLibrary.Array_Length` _outrownames))))
    (:`then`
      (bind (_enemyname _enemyhealth _armor _idleanimation _damagedanimation _deathanimation _attackanimation _blockanimation _healanimation _attack _defense _possibleactions) (break `/Game/Blueprints/DataTables/F_EnemyInfoStructure` _returnvalue))
      (`PaperFlipbookComponent.SetFlipbook` (`self.EnemySprite`) _idleanimation)
      (set `self.Name` _enemyname)
      (bind _output_get (set `self.CurrentHealth` _enemyhealth))
      (set `self.MaxHealth` _output_get)
      (set `self.Armor` _armor)
      (set `self.Attack` _attack)
      (set `self.Defense` _defense)
      (set `self.IdleFlipbook` _idleanimation)
      (set `self.DamagedFlipbook` _damagedanimation)
      (set `self.DeathFlipbook` _deathanimation)
      (set `self.Actions` _possibleactions))))

(fn `ResetAnimation`
  (`PaperFlipbookComponent.SetFlipbook` (`self.EnemySprite`) (`self.IdleFlipbook`)))

(fn `TakeEnemyTurn`
  (bind _keys (`BlueprintMapLibrary.Map_Keys` (`self.Actions`)))
  (`self.ApplyCardEffect` (`|GetArrayItem` _keys)))

(fn `UserConstructionScript`)